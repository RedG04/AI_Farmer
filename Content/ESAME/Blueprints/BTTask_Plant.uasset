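; BTTask_Plant is a behavior tree task in which a BP_Farmer pawn plants a BP_Plant.
; It spawns the plant at the farmer's location plus the forward vector multiplied component-wise by an X-only vector, so the offset lies only along world X.
; It then clears the HasSeeds blackboard key and finishes successfully.
; A failed cast to BP_Farmer stops execution without finishing the task.
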(event `self.ReceiveExecuteAI`
  (params (OwnerController :type "AIController Object Reference") (ControlledPawn :type "Pawn Object Reference"))
  (bind _asbp_farmer (cast `/Game/ESAME/NPC/BP_Farmer` ControlledPawn))
  (`|SpawnActorFromClass` "/Game/ESAME/Blueprints/BP_Plant.BP_Plant_C" (`KismetMathLibrary.Conv_VectorToTransform` (+ (`Actor.K2_GetActorLocation` _asbp_farmer) (* (`Actor.GetActorForwardVector` _asbp_farmer) (150.0 0.0 0.0)))) "Undefined" "MultiplyWithRoot" null (struct) null)
  (`BlackboardComponent.SetValueAsBool` (`AIBlueprintHelperLibrary.GetBlackboard` OwnerController) (`KismetStringLibrary.Conv_StringToName` "HasSeeds") false)
  (`self.FinishExecute` true))