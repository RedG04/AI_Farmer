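; AI controller for a turret that runs the BT_Turret behavior tree on BeginPlay.
; Perception updates write any sensed actor tagged "Enemy" into the TargetEnemy blackboard key and cancel the pending reset.
; When a stimulus is lost, a short timer calls ResetToPatroll, which clears TargetEnemy.
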(event `self.ReceiveBeginPlay`
  (`self.RunBehaviorTree` "/Game/ESAME/Blueprints/Turret/AI/BT_Turret.BT_Turret"))

(event `self.AIPerception.OnTargetPerceptionUpdated`
  (params (Actor :type "Actor Object Reference") (Stimulus :type "AIStimulus Structure"))
  (if (`.bSuccessfullySensed` (break `AIStimulus` Stimulus))
    (if (`self.ActorHasTag` Actor "Enemy")
      (`KismetSystemLibrary.K2_ClearTimer` null "ResetToPatroll")
      (`BlackboardComponent.SetValueAsObject` (`AIBlueprintHelperLibrary.GetBlackboard` null) "TargetEnemy" Actor)
      (else
        (`KismetSystemLibrary.PrintString` "Nope")))
    (else
      (`KismetSystemLibrary.K2_SetTimerDelegate` (delegate `ResetToPatroll`) 3.0))))

(event `ResetToPatroll`
  (`BlackboardComponent.SetValueAsObject` (`AIBlueprintHelperLibrary.GetBlackboard` null) "TargetEnemy" null))

(fn `UserConstructionScript`)