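; Behavior tree task that makes the farmer pick up the plant it is targeting.
; It reads the plant from the TargetActor blackboard key, destroys it, sets HasPlant on both the blackboard and the farmer, then updates the farmer's color.
; The task reports failure even after a successful pickup, and never finishes if either cast fails.
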(event `self.ReceiveExecuteAI`
  (params (OwnerController :type "AIController Object Reference") (ControlledPawn :type "Pawn Object Reference"))
  (bind _returnvalue (`AIBlueprintHelperLibrary.GetBlackboard` OwnerController))
  (bind _asbp_farmer (cast `/Game/ESAME/Blueprints/Farmer/NPC/BP_Farmer` ControlledPawn))
  (bind _asbp_plant (cast `/Game/ESAME/Blueprints/Farmer/BP_Plant` (`BlackboardComponent.GetValueAsObject` _returnvalue "TargetActor")))
  (`Actor.K2_DestroyActor` _asbp_plant)
  (`BlackboardComponent.SetValueAsBool` _returnvalue "HasPlant" true)
  (set `/Game/ESAME/Blueprints/Farmer/NPC/BP_Farmer.HasPlant` true _asbp_farmer)
  (`/Game/ESAME/Blueprints/Farmer/NPC/BP_Farmer.UpdateColor` _asbp_farmer)
  (`self.FinishExecute` false))