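; BP_Plant is a farm plant that grows from brown to mature green and then becomes takeable.
; On BeginPlay it starts a GrowTime timer, whose event sets IsMature, adds the Plant.Takeable gameplay tag and swaps the material.
; The mature plant then writes itself as TargetActor into the Blackboard of the AI referenced by BP_ThirdPersonGameMode, pushing itself to that agent as a target.
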(event `self.ReceiveBeginPlay`
  (`PrimitiveComponent.SetMaterial` (`self.StaticMesh`) 0 "/Game/ESAME/Material/Farmer/M_PlantBrown.M_PlantBrown")
  (`KismetSystemLibrary.K2_SetTimerDelegate` (delegate `Timer`) (`self.GrowTime`)))

(event `Timer`
  (set `self.IsMature` true)
  (`BlueprintGameplayTagLibrary.AddGameplayTag` (`self.PlantTags`) (struct :`TagName` "Plant.Takeable"))
  (`PrimitiveComponent.SetMaterial` (`self.StaticMesh`) 0 "/Game/ESAME/Material/Farmer/M_PlantGreen.M_PlantGreen")
  (bind _asbp_third_person_game_mode (cast `/Game/ThirdPerson/Blueprints/BP_ThirdPersonGameMode` (`GameplayStatics.GetGameMode`)))
  (`BlackboardComponent.SetValueAsObject` (`AIBlueprintHelperLibrary.GetBlackboard` (`/Game/ThirdPerson/Blueprints/BP_ThirdPersonGameMode.IA` _asbp_third_person_game_mode)) "TargetActor" self))

(fn `UserConstructionScript`)