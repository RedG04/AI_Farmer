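; BP_Farmer is the farmer NPC, whose material color shows whether it has a plant.
; On BeginPlay it creates a dynamic instance of M_Farmer on its mesh and registers itself as the IA reference on BP_ThirdPersonGameMode.
; UpdateColor sets the StateColor parameter to yellow or red based on HasPlant; nothing in this Blueprint calls it or changes that flag.
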(event `self.ReceiveBeginPlay`
  (`PrimitiveComponent.CreateDynamicMaterialInstance` (`self.Mesh`) 0 "/Game/ESAME/Material/Farmer/M_Farmer.M_Farmer" "None")
  (bind _asbp_third_person_game_mode (cast `/Game/ThirdPerson/Blueprints/BP_ThirdPersonGameMode` (`GameplayStatics.GetGameMode`)))
  (set `/Game/ThirdPerson/Blueprints/BP_ThirdPersonGameMode.IA` self _asbp_third_person_game_mode))

(fn `UpdateColor`
  (if (`self.HasPlant`)
    (`MeshComponent.SetColorParameterValueOnMaterials` (`self.Mesh`) "StateColor" (struct :`R` 1.0 :`G` 0.90211 :`A` 1.0))
    (else
      (`MeshComponent.SetColorParameterValueOnMaterials` (`self.Mesh`) "StateColor" (struct :`R` 1.0 :`G` 0.014145 :`B` 0.000127 :`A` 1.0)))))

(fn `UserConstructionScript`)